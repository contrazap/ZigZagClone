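; Floor spawner that builds a path of chained BP_Floor1 segments for an endless-runner-style track.
; On BeginPlay, it spawns an initial run, placing each segment at the previous one's Endpoint.
; A floor overlapping DestroyTrigger calls SpawnFloor and is destroyed after a short delay.
; SpawnFloor appends at the last Endpoint but then clears LastSpawnedFloor instead of storing the new floor, so later calls spawn nothing.
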(event `self.ReceiveBeginPlay`
  (`self.Initialize`))

(event `self.DestroyTrigger.OnComponentBeginOverlap`
  (params (OverlappedComponent :type "PrimitiveComponent Object Reference") (OtherActor :type "Actor Object Reference") (OtherComp :type "PrimitiveComponent Object Reference") (OtherBodyIndex :type Integer) (bFromSweep :type Boolean) (SweepResult :type "HitResult Structure (by ref)"))
  (bind _asbp_floor_1 (cast `/Game/Floors/Floor1/BP_Floor1` OtherActor))
  (`self.SpawnFloor`)
  (`KismetSystemLibrary.Delay` 2.0)
  (`self.K2_DestroyActor` _asbp_floor_1))

(fn `Initialize`
  (for _ (range 4)
    (`/Engine/EditorBlueprintResources/StandardMacros.IsValid` (`self.LastSpawnedFloor`)
      (:`Is Valid`
        (bind _returnvalue (`|SpawnActorFromClass` "/Game/Floors/Floor1/BP_Floor1.BP_Floor1_C" (`KismetMathLibrary.MakeTransform` (`SceneComponent.K2_GetComponentLocation` (`/Game/Floors/Floor1/BP_Floor1.Endpoint` (`self.LastSpawnedFloor`)))) "Undefined" "MultiplyWithRoot" null null))
        (set `self.LastSpawnedFloor` _returnvalue))
      (:`Is Not Valid`
        (bind _returnvalue_2 (`|SpawnActorFromClass` "/Game/Floors/Floor1/BP_Floor1.BP_Floor1_C" (`KismetMathLibrary.MakeTransform` (0.0 0.0 0.0)) "Undefined" "MultiplyWithRoot" null null))
        (set `self.LastSpawnedFloor` _returnvalue_2)))))

(fn `SpawnFloor`
  (`/Engine/EditorBlueprintResources/StandardMacros.IsValid` (`self.LastSpawnedFloor`)
    (:`Is Valid`
      (`|SpawnActorFromClass` "/Game/Floors/Floor1/BP_Floor1.BP_Floor1_C" (`KismetMathLibrary.MakeTransform` (`SceneComponent.K2_GetComponentLocation` (`/Game/Floors/Floor1/BP_Floor1.Endpoint` (`self.LastSpawnedFloor`)))) "Undefined" "MultiplyWithRoot" null null)
      (set `self.LastSpawnedFloor` null))))

(fn `UserConstructionScript`)