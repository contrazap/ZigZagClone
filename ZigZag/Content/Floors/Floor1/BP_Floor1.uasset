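; Floor actor for a zigzag game that slides its mesh each tick and carries a random set of coins.
; BeginPlay enables input, adds the mapping context, and spawns coins at a random, non-repeating subset of four spawn points, attached to the mesh.
; IA_Move flip-flops the movement vector between local X and Y, starting on X, which Tick applies as a swept offset without delta-time scaling.
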(event `self.ReceiveBeginPlay`
  (bind _returnvalue (`GameplayStatics.GetPlayerController` 0))
  (`self.EnableInput` _returnvalue)
  (bind _asbp_zig_zag_controller (cast `/Game/Blueprints/BP_ZigZagController` _returnvalue))
  (`EnhancedInputSubsystemInterface.AddMappingContext` (pcsubsystem `EnhancedInputLocalPlayerSubsystem` _asbp_zig_zag_controller) "/Game/Input/InputContext.InputContext" 0 (struct))
  (set `self.MovementVector` (`KismetMathLibrary.MakeVector` (* (`self.MoveOffset`) (`self.FloorSpeed`))))
  (bind _output_get (set `self.SpawnPoints` (`|MakeArray` (`self.SP1`) (`self.SP2`) (`self.SP3`) (`self.SP4`))))
  (bind _spawnindexarrout (`self.GetRandomSpawnPoints` (`KismetArrayLibrary.Array_Length` _output_get)))
  (for _array_element _spawnindexarrout
    (`self.SpawnCoins` (`SceneComponent.K2_GetComponentLocation` (`|GetArrayItem` (`self.SpawnPoints`) _array_element)))))

(event `self.ReceiveTick`
  (params (DeltaSeconds :type "Float (single-precision)"))
  (`SceneComponent.K2_AddLocalOffset` (`self.FloorMesh`) (`self.MovementVector`) true false))

(event `EnhancedInput|/Game/Input/IA_Move`
  (params (ActionValue :type Boolean) (ElapsedSeconds :type "Float (double-precision)") (TriggeredSeconds :type "Float (double-precision)") (InputAction :type "InputAction Object Reference" :default "/Game/Input/IA_Move.IA_Move"))
  (:`Triggered`
    (`/Engine/EditorBlueprintResources/StandardMacros.FlipFlop`
      (:`A`
        (set `self.MovementVector` (`KismetMathLibrary.MakeVector` 0.0 (* (`self.MoveOffset`) (`self.FloorSpeed`)))))
      (:`B`
        (set `self.MovementVector` (`KismetMathLibrary.MakeVector` (* (`self.MoveOffset`) (`self.FloorSpeed`))))))))

(fn `GetRandomSpawnPoints`
  (params (ArrayLength :type Integer))
  (returns (SpawnIndexArrOut :type "Array of Integer"))
  (locals (Counter :type Integer :default 0) (SpawnIndex :type "Array of Integer") (InputArrLen :type Integer))
  (set `local.InputArrLen` ArrayLength)
  (set `local.Counter` (`KismetMathLibrary.RandomIntegerInRange` 1 ArrayLength))
  (while (< (`KismetArrayLibrary.Array_Length` (`local.SpawnIndex`)) (`local.Counter`))
    (`KismetArrayLibrary.Array_AddUnique` (`local.SpawnIndex`) (`KismetMathLibrary.RandomIntegerInRange` 0 (- (`local.InputArrLen`) 1))))
  (return (`local.SpawnIndex`)))

(fn `SpawnCoins`
  (params (SpawnPointWorldLocation :type "Vector Structure"))
  (bind _returnvalue (`|SpawnActorFromClass` "/Game/Pickups/Coin/BP_Coin.BP_Coin_C" (`KismetMathLibrary.MakeTransform` SpawnPointWorldLocation) "Undefined" "MultiplyWithRoot" null null))
  (`self.K2_AttachToComponent` _returnvalue (`self.FloorMesh`) "None" "KeepWorld" "KeepRelative" "KeepRelative" true))

(fn `UserConstructionScript`)