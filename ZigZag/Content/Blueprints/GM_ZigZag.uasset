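; Game mode for ZigZag that spawns the player at a tagged spawn point, plays music, and manages the menu, HUD, pausing, coin count and death.
; A running flag on the game instance persists across level reloads, so restarting after death reopens Level1 straight into gameplay instead of the menu.
; Coins collected update a high score, which is saved to a save slot whenever beaten and loaded on BeginPlay.
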(event `self.ReceiveBeginPlay`
  (`GameplayStatics.PlaySound2D` "/Game/Audio/SC_ZigZag.SC_ZigZag" 1.0 1.0 0.0 null null)
  (bind _outactors (`GameplayStatics.GetAllActorsWithTag` "PlayerSpawnPoint"))
  (bind _returnvalue (`|SpawnActorFromClass` "/Game/Player/BP_Player.BP_Player_C" (`KismetMathLibrary.MakeTransform` (`self.K2_GetActorLocation` (`|GetArrayItem` _outactors))) "Undefined" "MultiplyWithRoot" null null))
  (set `self.PlayerRef` _returnvalue)
  (bind _returnvalue_2 (`|CreateWidget` "/Game/UI/WB_HUD.WB_HUD_C"))
  (set `self.HudRef` _returnvalue_2)
  (bind _returnvalue_3 (`|CreateWidget` "/Game/UI/WB_Menu.WB_Menu_C"))
  (set `self.MenuRef` _returnvalue_3)
  (`self.LoadSaveGame`)
  (bind _asgi_zig_zag (cast `/Game/Blueprints/GI_ZigZag` (`GameplayStatics.GetGameInstance`)))
  (if (`/Game/Blueprints/GI_ZigZag.IsGameRunning` _asgi_zig_zag)
    (`WidgetBlueprintLibrary.SetInputMode_GameOnly` (`GameplayStatics.GetPlayerController` 0))
    (`UserWidget.AddToViewport` (`self.HudRef`) 0)
    (else
      (`self.ShowMenu`))))

(event `IncrementCoins`
  (bind _output_get (set `self.CoinsCollected` (+ (`self.CoinsCollected`) 1)))
  (if (> _output_get (`self.HighScore`))
    (set `self.HighScore` (`self.CoinsCollected`))
    (bind _asbp_save_game (cast `/Game/Blueprints/BP_SaveGame` (`self.SaveGameObject`)))
    (set `/Game/Blueprints/BP_SaveGame.HighScore` (`self.HighScore`) _asbp_save_game)
    (`GameplayStatics.SaveGameToSlot` (`self.SaveGameObject`) "Slot1")))

(event `HandlePlayerDeath`
  (set `self.IsPlayerDead` true)
  (`self.ShowMenu`))

(event `ShowMenu`
  (bind _returnvalue (`GameplayStatics.GetPlayerController` 0))
  (`GameplayStatics.SetGamePaused` true)
  (`Widget.RemoveFromParent` (`self.HudRef`))
  (`UserWidget.AddToViewport` (`self.MenuRef`) 0)
  (`WidgetBlueprintLibrary.SetInputMode_UIOnlyEx` _returnvalue (`self.MenuRef`))
  (set `PlayerController.bShowMouseCursor` true _returnvalue))

(event `HandleStart`
  (bind _returnvalue (`GameplayStatics.GetPlayerController` 0))
  (bind _asgi_zig_zag (cast `/Game/Blueprints/GI_ZigZag` (`GameplayStatics.GetGameInstance`)))
  (if (`/Game/Blueprints/GI_ZigZag.IsGameRunning` _asgi_zig_zag)
    (if (`self.IsPlayerDead`)
      (`GameplayStatics.OpenLevel` "Level1")
      (else
        (`Widget.RemoveFromParent` (`self.MenuRef`) :!label _label)
        (`UserWidget.AddToViewport` (`self.HudRef`) 0)
        (`WidgetBlueprintLibrary.SetInputMode_GameOnly` _returnvalue)
        (`GameplayStatics.SetGamePaused` false)
        (set `PlayerController.bShowMouseCursor` false _returnvalue)))
    (else
      (set `/Game/Blueprints/GI_ZigZag.IsGameRunning` true _asgi_zig_zag)
      (goto _label))))

(fn `LoadSaveGame`
  (bind _returnvalue (`GameplayStatics.DoesSaveGameExist` "Slot1"))
  (if _returnvalue
    (bind _returnvalue_2 (`GameplayStatics.LoadGameFromSlot` "Slot1"))
    (`/Engine/EditorBlueprintResources/StandardMacros.IsValid` _returnvalue_2
      (:`Is Valid`
        (bind _output_get (set `self.SaveGameObject` _returnvalue_2))
        (bind _asbp_save_game (cast `/Game/Blueprints/BP_SaveGame` _output_get))
        (set `self.HighScore` (`/Game/Blueprints/BP_SaveGame.HighScore` _asbp_save_game))))
    (else
      (bind _returnvalue_3 (`GameplayStatics.CreateSaveGameObject` "/Game/Blueprints/BP_SaveGame.BP_SaveGame_C"))
      (`/Engine/EditorBlueprintResources/StandardMacros.IsValid` _returnvalue_3
        (:`Is Valid`
          (set `self.SaveGameObject` _returnvalue_3))))))

(fn `UserConstructionScript`)